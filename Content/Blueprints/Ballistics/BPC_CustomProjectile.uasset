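; Bullet component that moves its owning actor by per-frame line traces, simulating penetration and ricochet until its lifespan ends.
; A physical-material data table drives penetration odds from speed and angle, plus energy lost through thickness, measured by tracing back from beyond the hit actor.
; Ricochets mirror velocity at half speed; both outcomes randomly vary trajectory and spawn surface-based effects.
; Gravity adjusts only vertical velocity, and optional debug lines are colored by speed.
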(event `self.ReceiveBeginPlay`
  (bind _returnvalue (`self.GetOwner`))
  (set `self.Velocity` (* (`Actor.GetActorForwardVector` _returnvalue) (`self.BulletSpeed`)))
  (set `self.StartPos` (`Actor.K2_GetActorLocation` _returnvalue))
  (set `self.bIsInitialized?` true)
  (`KismetSystemLibrary.Delay` (`self.BulletLifeSpan`))
  (`Actor.K2_DestroyActor` (`self.GetOwner`)))

(event `self.ReceiveTick`
  (params (DeltaSeconds :type "Float (single-precision)"))
  (bind _outhit (`self.OutHit`))
  (if (`self.bIsInitialized?`)
    (set `self.DeltaTime` DeltaSeconds)
    (set `self.StartPos` (`Actor.K2_GetActorLocation` (`self.GetOwner`)))
    (set `self.LastPos` (+ (`self.StartPos`) (* (`self.Velocity`) (`self.DeltaTime`))))
    (bind (_outhit_2 _returnvalue) (`KismetSystemLibrary.LineTraceSingle` (`self.StartPos`) (`self.LastPos`) "TraceTypeQuery1" false (`|MakeArray` (`self.ActorToIgnore`)) "None" true (struct :`R` 1.0 :`A` 1.0) (struct :`G` 1.0 :`A` 1.0) 10.0))
    (if (`self.bIsDebugLineVisible?`)
      (`KismetSystemLibrary.DrawDebugLine` (`self.StartPos`) (select `bool` _returnvalue :`false` (`self.LastPos`) :`true` (`.ImpactPoint` (`GameplayStatics.BreakHitResult` _outhit_2))) (`self.GetTraceColor`) 10.0))
    (if _returnvalue
      (bind _output_get (set `self.OutHit` _outhit_2))
      (if (`self.WhetherToPenetrate` (`self.Velocity`) (`self.OutHit`))
        (`self.BulletImpact` _output_get)
        (bind (_bhit_ _exitlocation _surfacenormal _outhit_3) (`self.ComputeExitLocation` (`KismetMathLibrary.Normal` (`self.Velocity`)) (`self.OutHit`)))
        (if _bhit_
          (bind _returnvalue_2 (`self.CalculateFinalVelocity` (`self.Velocity`) _exitlocation (`self.OutHit`)))
          (if (> _returnvalue_2 0.0)
            (set `self.ActorToIgnore` (`.HitActor` (`GameplayStatics.BreakHitResult` (`self.OutHit`))))
            (`self.BulletImpact` _outhit_3)
            (`Actor.K2_SetActorLocation` (`self.GetOwner`) _exitlocation false false)
            (bind _output_get_2 (set `self.Velocity` (`self.ComputeGravityAndDeceleration` (* (`KismetMathLibrary.Normal` (`self.Velocity`)) _returnvalue_2))))
            (`self.VaryTrajectory` _surfacenormal _output_get_2)
            (else
              (`Actor.K2_DestroyActor` (`self.GetOwner`)))))
        (else
          (`self.HitImpact` _outhit true)
          (bind (_startpoint _velocity _impactnormal) (`self.ComputeRicochet` _outhit))
          (set `self.ActorToIgnore` (`.HitActor` (`GameplayStatics.BreakHitResult` _outhit)))
          (`Actor.K2_SetActorLocation` (`self.GetOwner`) _startpoint false false)
          (bind _output_get_3 (set `self.Velocity` (`self.ComputeGravityAndDeceleration` _velocity)))
          (`self.VaryTrajectory` _impactnormal _output_get_3)))
      (else
        (`Actor.K2_SetActorLocation` (`self.GetOwner`) (`self.LastPos`) false false)
        (set `self.Velocity` (`self.ComputeGravityAndDeceleration` (`self.Velocity`)))))))

(fn `AngleBetweenVectors`
  (params (V1 :type "Vector Structure") (V2 :type "Vector Structure"))
  (returns (ReturnValue :type "Float (double-precision)"))
  (return (`KismetMathLibrary.DegAcos` (`KismetMathLibrary.Dot_VectorVector` (`KismetMathLibrary.Normal` V1) (`KismetMathLibrary.Normal` V2)))))

(fn `BulletImpact`
  (params (HitResult :type "HitResult Structure"))
  (bind (_bblockinghit _binitialoverlap _time _distance _location _impactpoint _normal _impactnormal) (`GameplayStatics.BreakHitResult` HitResult))
  (bind _returnvalue (`GameplayStatics.SpawnDecalAtLocation` (`self.DecalMaterial`) (`self.DecalSize`) _location (`KismetMathLibrary.MakeRotFromX` _impactnormal) (`self.DecalLifeSpan`)))
  (`DecalComponent.SetFadeScreenSize` _returnvalue (`self.DecalFadeScreenSize`))
  (`self.HitImpact` (`local.HitResult`)))

(fn `CalculateFinalVelocity`
  (params (InVelocity :type "Vector Structure") (ExitLocation :type "Vector Structure") (OutHit :type "HitResult Structure"))
  (returns (ReturnValue :type "Float (double-precision)"))
  (bind (_bblockinghit _binitialoverlap _time _distance _location _impactpoint _normal _impactnormal _physmat) (`GameplayStatics.BreakHitResult` OutHit))
  (bind _returnvalue (* 0.5 (`self.BulletMass`) (`KismetMathLibrary.VSizeSquared` (`local.InVelocity`))))
  (bind _returnvalue_2 (`|GetDataTableRow` "/Game/Blueprints/Ballistics/MaterialData.MaterialData" (`KismetStringLibrary.Conv_StringToName` (`KismetSystemLibrary.GetObjectName` _physmat)))
    (:`then`
      (bind _returnvalue_3 (* (`KismetMathLibrary.Vector_Distance` (`local.ExitLocation`) _impactpoint) _returnvalue (`.JoulesPerCM_4_62072558494517F9E2AFCB80277C614F` (break `/Game/Blueprints/Ballistics/PenetrationData` _returnvalue_2))))
      (return (`KismetMathLibrary.Sqrt` (/ (- _returnvalue (select `bool` (> _returnvalue_3 _returnvalue) :`false` _returnvalue_3 :`true` _returnvalue)) (* (`self.BulletMass`) 0.5)))))
    (:`RowNotFound`
      (return (`KismetMathLibrary.VSize` (`local.InVelocity`))))))

(fn `ComputeExitLocation`
  (params (Direction :type "Vector Structure") (HitResult :type "HitResult Structure"))
  (returns (`bHit?` :type Boolean) (ExitLocation :type "Vector Structure") (SurfaceNormal :type "Vector Structure") (OutHit :type "HitResult Structure"))
  (locals (TraceDistance :type "Float (double-precision)") (TraceStart :type "Vector Structure") (TraceEnd :type "Vector Structure") (IgnoreList :type "Array of Actor Object Reference") (InitialHitActor :type "Actor Object Reference"))
  (bind (_bblockinghit _binitialoverlap _time _distance _location _impactpoint _normal _impactnormal _physmat _hitactor) (`GameplayStatics.BreakHitResult` HitResult))
  (bind (_origin _boxextent) (`Actor.GetActorBounds` _hitactor true true))
  (set `local.InitialHitActor` _hitactor)
  (bind _output_get (set `local.TraceDistance` (* (`KismetMathLibrary.FMax` (.x _boxextent) (.y _boxextent) (.z _boxextent)) 4.0)))
  (bind _output_get_2 (set `local.TraceStart` (+ (* (`local.Direction`) _output_get) _impactpoint)))
  (set `local.TraceEnd` (+ _output_get_2 (* (`local.Direction`) (* (`local.TraceDistance`) -1.0))))
  (bind (_outhit _returnvalue) (`KismetSystemLibrary.LineTraceSingle` (`local.TraceStart`) (`local.TraceEnd`) "TraceTypeQuery1" false (`local.IgnoreList`) "None" true (struct :`R` 1.0 :`G` 0.756324 :`A` 1.0) (struct :`G` 1.0 :`B` 0.883942 :`A` 1.0) :!label _label))
  (if _returnvalue
    (bind (_bblockinghit_2 _binitialoverlap_2 _time_2 _distance_2 _location_2 _impactpoint_2 _normal_2 _impactnormal_2 _physmat_2 _hitactor_2) (`GameplayStatics.BreakHitResult` _outhit))
    (if (!= _hitactor_2 (`local.InitialHitActor`))
      (`KismetArrayLibrary.Array_Add` (`local.IgnoreList`) _hitactor_2)
      (set `local.TraceStart` _impactpoint_2)
      (goto _label)
      (else
        (return true _impactpoint_2 _impactnormal_2 _outhit)))
    (else
      (return false (0.0 0.0 0.0) _impactnormal_2))))

(fn `ComputeGravityAndDeceleration`
  (params (Velocity :type "Vector Structure"))
  (returns (ReturnValue :type "Vector Structure"))
  (return (+ Velocity (* (`KismetMathLibrary.MakeVector` 0.0 0.0 (+ (`self.DragForce` (`self.AirDensity`) (`self.BulletSpeed`) (`self.DragCoefficiency`) (`self.CrossSection`)) (* (* (`self.Gravity`) 100.0) (`self.BulletMass`) -1.0))) (`self.DeltaTime`)))))

(fn `ComputeRicochet`
  (params (Hit :type "HitResult Structure"))
  (returns (StartPoint :type "Vector Structure") (Velocity :type "Vector Structure") (ImpactNormal :type "Vector Structure"))
  (bind (_bblockinghit _binitialoverlap _time _distance _location _impactpoint _normal _impactnormal) (`GameplayStatics.BreakHitResult` Hit))
  (bind _velocity (`self.Velocity`))
  (bind _returnvalue (`KismetMathLibrary.VSize` _velocity))
  (return (+ _impactpoint _impactnormal) (`KismetMathLibrary.MirrorVectorByNormal` (* (`KismetMathLibrary.Normal` _velocity) (- _returnvalue (/ _returnvalue 2.0))) _impactnormal) _impactnormal))

(fn `DetermineHitEffects`
  (params (Surface :type "EPhysicalSurface Enum" :default "SurfaceType_Default") (`bRicochet?` :type Boolean))
  (returns (HitSFX :type "SoundBase Object Reference") (ParticleSystem :type "ParticleSystem Object Reference"))
  (return (select `bool` (`local.bRicochet?`) :`false` (select `EPhysicalSurface` Surface :`SurfaceType_Default` "/Game/Blueprints/Ballistics/FreesoundSFX/Ground_Cue.Ground_Cue" :`SurfaceType1` "/Game/Blueprints/Ballistics/FreesoundSFX/Wood_Cue.Wood_Cue" :`SurfaceType2` "/Game/Blueprints/Ballistics/FreesoundSFX/Metal_Cue.Metal_Cue" :`SurfaceType3` "/Game/Blueprints/Ballistics/FreesoundSFX/Gore_Cue.Gore_Cue" :`SurfaceType4` "/Game/Blueprints/Ballistics/FreesoundSFX/Concrete_Cue.Concrete_Cue" :`SurfaceType5` "/Game/Blueprints/Ballistics/FreesoundSFX/Ground_Cue.Ground_Cue" :!type "SoundBase Object Reference") :`true` "/Game/Blueprints/Ballistics/FreesoundSFX/Ricochet_Cue.Ricochet_Cue") (select `EPhysicalSurface` Surface :`SurfaceType_Default` "/Game/Realistic_Starter_VFX_Pack_Vol2/Particles/Hit/P_Default.P_Default" :`SurfaceType1` "/Game/Realistic_Starter_VFX_Pack_Vol2/Particles/Hit/P_Brick.P_Brick" :`SurfaceType2` "/Game/Realistic_Starter_VFX_Pack_Vol2/Particles/Hit/P_Default.P_Default" :`SurfaceType4` "/Game/Realistic_Starter_VFX_Pack_Vol2/Particles/Hit/P_Concrete.P_Concrete" :`SurfaceType5` "/Game/Realistic_Starter_VFX_Pack_Vol2/Particles/Hit/P_Asphalt.P_Asphalt" :!type "ParticleSystem Object Reference")))

(fn `GetTraceColor`
  (returns (ReturnValue :type "LinearColor Structure"))
  (bind _returnvalue (/ (`KismetMathLibrary.VSize` (`self.Velocity`)) (`self.BulletSpeed`)))
  (if (> _returnvalue 0.75)
    (return (`KismetMathLibrary.LinearColorLerp` (struct :`R` 0.223228 :`B` 0.001518 :`A` 1.0) (struct :`R` 0.005182 :`A` 1.0) (* (- _returnvalue 0.75) 4.0)))
    (elif (> _returnvalue 0.5)
      (return (`KismetMathLibrary.LinearColorLerp` (struct :`R` 1.0 :`G` 0.577581 :`A` 1.0) (struct :`R` 0.223228 :`B` 0.001518 :`A` 1.0) (* (- _returnvalue 0.5) 4.0)))
      (elif (> _returnvalue 0.25)
        (return (`KismetMathLibrary.LinearColorLerp` (struct :`G` 1.0 :`B` 0.270498 :`A` 1.0) (struct :`R` 1.0 :`G` 0.577581 :`A` 1.0) (* (- _returnvalue 0.25) 4.0)))
        (else
          (return (`KismetMathLibrary.LinearColorLerp` (struct :`R` 0.708376 :`G` 1.0 :`B` 0.701102 :`A` 1.0) (struct :`G` 1.0 :`B` 0.270498 :`A` 1.0) (* _returnvalue 4.0))))))))

(fn `HitImpact`
  (params (HitResult :type "HitResult Structure") (`bRicochet?` :type Boolean))
  (bind (_hitsfx _particlesystem) (`self.DetermineHitEffects` (`PhysicalMaterial.SurfaceType` HitResult_PhysMat) `bRicochet?`))
  (`GameplayStatics.SpawnSoundAtLocation` _hitsfx HitResult_Location (struct) 1.0 1.0 0.0 null null)
  (`GameplayStatics.SpawnEmitterAtLocation` _particlesystem HitResult_Location (`KismetMathLibrary.MakeRotFromX` HitResult_ImpactNormal)))

(fn `VaryTrajectory`
  (params (SurfaceNormal :type "Vector Structure") (ImpactVelocity :type "Vector Structure"))
  (locals (InitialAnswer :type "Vector Structure"))
  (bind _velocity (`self.Velocity`))
  (bind _output_get (set `local.InitialAnswer` (* (`KismetMathLibrary.RandomUnitVectorInConeInRadians` _velocity (`KismetMathLibrary.MapRangeClamped` (`KismetMathLibrary.VSize` ImpactVelocity) 20000.0 60000.0 0.096 0.149)) (`KismetMathLibrary.VSize` _velocity))))
  (bind _returnvalue (`self.AngleBetweenVectors` SurfaceNormal _output_get))
  (if (>= _returnvalue 90.0)
    (set `self.Velocity` (`KismetMathLibrary.GreaterGreater_VectorRotator` (`local.InitialAnswer`) (* (`KismetMathLibrary.NormalizedDeltaRotator` (`KismetMathLibrary.MakeRotFromX` SurfaceNormal) (`KismetMathLibrary.MakeRotFromX` (`local.InitialAnswer`))) (- 1.0 (/ _returnvalue 90.0)))))
    (else
      (set `self.Velocity` (`local.InitialAnswer`))))
  (return))

(fn `WhetherToPenetrate`
  (params (Velocity :type "Vector Structure") (OutHit :type "HitResult Structure"))
  (returns (Result :type Boolean))
  (bind (_bblockinghit _binitialoverlap _time _distance _location _impactpoint _normal _impactnormal _physmat) (`GameplayStatics.BreakHitResult` OutHit))
  (bind _velocity (`self.Velocity`))
  (bind _returnvalue (`|GetDataTableRow` "/Game/Blueprints/Ballistics/MaterialData.MaterialData" (`KismetStringLibrary.Conv_StringToName` (`KismetSystemLibrary.GetObjectName` _physmat)))
    (:`then`
      (bind (_joulespercm _impactanglegradient _impactanglezintercept _velocitygradient _velocityzintercept _minvelocitytopenetrate) (break `/Game/Blueprints/Ballistics/PenetrationData` _returnvalue))
      (return (and (> (* (`KismetMathLibrary.FClamp` (+ (* (`KismetMathLibrary.VSize` _velocity) _velocitygradient) _velocityzintercept)) (`KismetMathLibrary.FClamp` (+ (* _impactanglegradient (`self.AngleBetweenVectors` (* _impactnormal -1.0) (`KismetMathLibrary.Normal` _velocity))) _impactanglezintercept))) (`KismetMathLibrary.RandomFloatInRange` 0.0 1.0)) (> (/ (`KismetMathLibrary.VSize` (`self.Velocity`)) (`self.BulletSpeed`)) _minvelocitytopenetrate))))
    (:`RowNotFound`
      (return false))))