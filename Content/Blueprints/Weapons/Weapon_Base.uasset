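; Base weapon Blueprint that provides shared setup and hitscan tracing, with stub events for firing, reloading and stowing.
; It caches the parent first-person character on BeginPlay, passes its ADS offset on Equip, and applies mesh and material at construction.
; FireHitscan traces from the camera within a spread cone, stores that hit, then traces from the muzzle toward the aim point with optional debug drawing.
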(event `self.ReceiveBeginPlay`
  ;[1 1 1] Get Player Reference
  (bind _asbp_first_person_character (cast `/Game/FirstPerson/Blueprints/BP_FirstPersonCharacter` (`self.GetParentActor`)))
  (set `self.PlayerReference` _asbp_first_person_character))

(event `Equip`
  ;[0.05098 0.05098 0.05098] Events
  ;;[1 1 1] Update Player ADS Offset
  (set `/Game/FirstPerson/Blueprints/BP_FirstPersonCharacter.ADS_Offset` (`self.ADS_Offset`) (`self.PlayerReference`)))

(event `Stow`
  ;[0.05098 0.05098 0.05098] Events
)

(event `Fire`
  ;[0.05098 0.05098 0.05098] Events
)

(event `StopFire`
  ;[0.05098 0.05098 0.05098] Events
)

(event `Reload`
  ;[0.05098 0.05098 0.05098] Events
)

(event `CancelReload`
  ;[0.05098 0.05098 0.05098] Events
)

(fn `Fire_Hitscan`
  (params (DrawDebug :type Boolean :default true))
  (locals (HitInfoL :type "HitResult Structure"))
  (bind _firstpersoncamera (`/Game/FirstPerson/Blueprints/BP_FirstPersonCharacter.FirstPersonCamera` (`self.PlayerReference`)))
  (bind _returnvalue (`SceneComponent.K2_GetComponentLocation` _firstpersoncamera))
  (bind _returnvalue_2 (`KismetMathLibrary.RandomUnitVectorInConeInDegrees` (`SceneComponent.GetForwardVector` _firstpersoncamera) (`self.Spread`)))
  ;[1 1 1] Trace From Center Screen to Max Weapon Range
  (bind (_outhit _returnvalue_3) (`KismetSystemLibrary.LineTraceSingle` _returnvalue (+ _returnvalue (* _returnvalue_2 (`self.Range`))) "TraceTypeQuery1" false (`|MakeArray` (`self.PlayerReference`) :!type "Actor Object Reference")))
  ;[1 1 1] Trace From Weapon Muzzle to Center Trace Hit Location
  (set `local.HitInfoL` _outhit)
  (bind (_bblockinghit _binitialoverlap _time _distance _location _impactpoint _normal _impactnormal _physmat _hitactor _hitcomponent _hitbonename _bonename _hititem _elementindex _faceindex _tracestart _traceend) (`GameplayStatics.BreakHitResult` _outhit))
  (`KismetSystemLibrary.LineTraceSingle` (`SceneComponent.GetSocketLocation` (`self.Weapon_Mesh`) "Muzzle") (`KismetMathLibrary.SelectVector` (+ _location (* _returnvalue_2 10.0)) _traceend _returnvalue_3) "TraceTypeQuery1" false (`|MakeArray` (`self.PlayerReference`) :!type "Actor Object Reference") (select `bool` (`local.DrawDebug`) :`true` "ForDuration" :!type "EDrawDebugTrace Enum")))

(fn `UserConstructionScript`
  (bind _weapon_mesh (`self.Weapon_Mesh`))
  (`SkeletalMeshComponent.SetSkeletalMeshAsset` _weapon_mesh (`self.Mesh`))
  (`PrimitiveComponent.SetMaterial` _weapon_mesh 0 (`self.Material`)))