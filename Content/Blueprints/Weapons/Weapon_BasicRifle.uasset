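; Basic rifle weapon Blueprint that handles firing, reloading and reload cancelling through the player's first-person mesh.
; Fire, blocked while reloading, plays a montage and spawns an actor at the muzzle socket; the FireHitscan call is disconnected.
; Reload exits ADS and holds a Reloading flag until montage blend-out, or one second after interruption.
; CancelReload stops the reload montage and weapon mesh animation.
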(event `self.Fire`
  (bind (_returnvalue_location _returnvalue_rotation) (`KismetMathLibrary.BreakTransform` (`SceneComponent.GetSocketTransform` (`self.Weapon_Mesh`) "Muzzle" "RTS_World")))
  (if (not (`self.Reloading?`))
    ;[1 0 0.9141] Play Weapon Fire Animation
    (`|PlayMontage` (`/Game/FirstPerson/Blueprints/BP_FirstPersonCharacter.FirstPersonMesh` (`self.PlayerReference`)) "/Game/Animations/FirstPerson/FP_Fire_Montage.FP_Fire_Montage"
      (:`then`
        ;[0 0.4844 1] Fire Hitscan
        (`|SpawnActorFromClass` "/Game/Blueprints/Ballistics/BP_Bullet.BP_Bullet_C" (`KismetMathLibrary.MakeTransform` _returnvalue_location _returnvalue_rotation) "AlwaysSpawn" "OverrideRootScale" null null)))))

(event `self.Reload`
  (bind _playerreference (`self.PlayerReference`))
  (if (not (`self.Reloading?`))
    (set `self.Reloading?` true)
    (`/Game/FirstPerson/Blueprints/BP_FirstPersonCharacter.Exit ADS` _playerreference false)
    (`|PlayMontage` (`/Game/FirstPerson/Blueprints/BP_FirstPersonCharacter.FirstPersonMesh` _playerreference) "/Game/Animations/FirstPerson/FP_Reload_Montage.FP_Reload_Montage"
      (:`OnBlendOut`
        (set `self.Reloading?` false))
      (:`OnInterrupted`
        (`KismetSystemLibrary.Delay` 1.0)
        (set `self.Reloading?` false)))))

(event `self.CancelReload`
  (`AnimInstance.Montage_Stop` (`SkeletalMeshComponent.GetAnimInstance` (`/Game/FirstPerson/Blueprints/BP_FirstPersonCharacter.FirstPersonMesh` (`self.PlayerReference`))) 0.25 "/Game/Animations/FirstPerson/FP_Reload_Montage.FP_Reload_Montage")
  (`SkeletalMeshComponent.Stop` (`self.Weapon_Mesh`)))

(fn `UserConstructionScript`
  (`parent.UserConstructionScript`))